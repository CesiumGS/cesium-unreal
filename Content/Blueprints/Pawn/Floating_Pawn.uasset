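; Free-flying pawn that adjusts its movement speed and toggles debug and utility widgets.
; Mouse wheel up and down multiply or divide the Floating Pawn Movement max speed by increment and decrement factors.
; Two input actions create or remove the profiling and time-of-day widgets, showing the mouse cursor while opening one and hiding it when closing.
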(event `Key|MouseScrollUp`
  (params (Key :type "Key Structure"))
  (bind _movementcomponent (`self.MovementComponent`))
  (:`Pressed`
    (bind _asfloating_pawn_movement (cast `FloatingPawnMovement` _movementcomponent))
    (set `FloatingPawnMovement.MaxSpeed` (* (`MovementComponent.GetMaxSpeed` _movementcomponent) (`self.Increment`)) _asfloating_pawn_movement)))

(event `Key|MouseScrollDown`
  (params (Key :type "Key Structure"))
  (bind _movementcomponent (`self.MovementComponent`))
  (:`Pressed`
    (bind _asfloating_pawn_movement (cast `FloatingPawnMovement` _movementcomponent))
    (set `FloatingPawnMovement.MaxSpeed` (/ (`MovementComponent.GetMaxSpeed` _movementcomponent) (`self.Decrement`)) _asfloating_pawn_movement)))

(event `InputAction|ToggleProfilingWidget`
  (params (Key :type "Key Structure"))
  (:`Pressed`
    (`/Engine/EditorBlueprintResources/StandardMacros.IsValid` (`self.ProfilingWidget`)
      (:`Is Valid`
        (`Widget.RemoveFromParent` (`self.ProfilingWidget`))
        (set `self.ProfilingWidget` null)
        (set `PlayerController.bShowMouseCursor` false (`GameplayStatics.GetPlayerController` 0)))
      (:`Is Not Valid`
        (bind _returnvalue (`|CreateWidget` "/Game/Blueprints/Pawn/BPW_Profiling.BPW_Profiling_C"))
        (bind _output_get (set `self.ProfilingWidget` _returnvalue))
        (`UserWidget.AddToViewport` _output_get 0)
        (set `PlayerController.bShowMouseCursor` true (`GameplayStatics.GetPlayerController` 0))))))

(event `InputAction|ToggleTODWidget`
  (params (Key :type "Key Structure"))
  (:`Pressed`
    (`/Engine/EditorBlueprintResources/StandardMacros.IsValid` (`self.TODWidget`)
      (:`Is Valid`
        (`Widget.RemoveFromParent` (`self.TODWidget`))
        (set `self.TODWidget` null)
        (set `PlayerController.bShowMouseCursor` false (`GameplayStatics.GetPlayerController` 0)))
      (:`Is Not Valid`
        (bind _returnvalue (`|CreateWidget` "/Game/Blueprints/Pawn/BPW_TimeOfDay.BPW_TimeOfDay_C"))
        (bind _output_get (set `self.TODWidget` _returnvalue))
        (`UserWidget.AddToViewport` _output_get 0)
        (set `PlayerController.bShowMouseCursor` true (`GameplayStatics.GetPlayerController` 0))))))

(fn `UserConstructionScript`)