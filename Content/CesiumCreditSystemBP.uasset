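; Credit system actor Blueprint for Cesium that displays data credits in a screen widget.
; On BeginPlay it creates a ScreenCredits widget, clears its HTML and adds it to the viewport.
; Each Tick, when CreditsUpdated is set, it pushes the credits HTML and on-screen visibility flag to the widget.
; The separate on-screen HTML updates only while on-screen display is enabled.
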(event `self.ReceiveBeginPlay`
  (`parent.ReceiveBeginPlay`)
  (bind _returnvalue (`|CreateWidget` "/CesiumForUnreal/ScreenCredits.ScreenCredits_C"))
  (bind _output_get (set `self.ScreenCreditsObj` _returnvalue))
  (`/CesiumForUnreal/ScreenCredits.UpdateHtml` _output_get "")
  (`UserWidget.AddToViewport` _output_get 0))

(event `self.ReceiveTick`
  (params (DeltaSeconds :type "Float (single-precision)"))
  (`parent.ReceiveTick` DeltaSeconds)
  (if (`self.CreditsUpdated`)
    (`/CesiumForUnreal/ScreenCredits.UpdateHtml` (`self.ScreenCreditsObj`) (`self.Credits`))
    (set `/CesiumForUnreal/ScreenCredits.ShowOnScreenCredits` (`self.DisplayOnScreenCredits`) (`self.ScreenCreditsObj`))
    (if (`self.DisplayOnScreenCredits`)
      (`/CesiumForUnreal/ScreenCredits.UpdateOn-ScreenHtml` (`self.ScreenCreditsObj`) (`self.OnScreenCredits`)))))

(fn `UserConstructionScript`)